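; BP_Zombie_Spawner spawns BP_TestZombie actors at its own location, starting on BeginPlay.
; SpawnNewZombie recurses after a 15-second delay, repeating the wait while the box overlap flag reports a zombie in the spawn area.
; Begin and end overlaps set a single boolean rather than counting occupants.
; ActiveZombies only increments here, so the loop stops for good once it exceeds the cap of five.
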(event OnComponentBeginOverlap(Box)
  (params (OverlappedComponent :type Primitive%20Component%20Object%20Reference) (OtherActor :type Actor%20Object%20Reference) (OtherComp :type Primitive%20Component%20Object%20Reference) (OtherBodyIndex :type Integer) (bFromSweep :type Boolean) (SweepResult :type Hit%20Result%20Structure%20%28by%20ref%29))
  (Utilities|Casting|CastToBP_TestZombie OtherActor)
  (Variables|Default|SetzombieInRadius true))

(event OnComponentEndOverlap(Box)
  (params (OverlappedComponent :type Primitive%20Component%20Object%20Reference) (OtherActor :type Actor%20Object%20Reference) (OtherComp :type Primitive%20Component%20Object%20Reference) (OtherBodyIndex :type Integer))
  (Utilities|Casting|CastToBP_TestZombie OtherActor)
  (Variables|Default|SetzombieInRadius false))

(event Custom|Spawn%20New%20Zombie
  (if (<= (Variables|Default|GetactiveZombies) 5)
    (Game|SpawnActorfromClass "/Game/Blueprints/BP_TestZombie.BP_TestZombie_C" (Math|Transform|MakeTransform (Transformation|GetWorldLocation (Variables|Default|GetDefaultSceneRoot))) "Undefined" "MultiplyWithRoot" 0 0)
    (Math|Integer|IncrementInt (Variables|Default|GetactiveZombies)
      (:%20%20
        (Utilities|FlowControl|Delay 15.0 :!label _label)
        (if (Variables|Default|GetzombieInRadius)
          (goto _label)
          (else
            (CallFunction|SpawnNewZombie)))))))

(event EventBeginPlay
  (CallFunction|SpawnNewZombie))

(fn ConstructionScript)