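; BP_TestZombie is an enemy AI zombie that roams, hunts the player and deals repeated damage while overlapping its HitBox.
; AIMoveTo drives looping random roaming, faster chases from PawnSensing sightings, and moves to AIPerception gunshot stimuli.
; SoundInvestigate, once set, is never cleared here, so roaming stops re-looping.
; Damage reduces clamped health; death stops movement, spawns BP_ZombieSou and possibly MP5 or pistol ammo, then destroys the actor.
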(event OnSeePawn(PawnSensing)
  (params (Pawn :type Pawn%20Object%20Reference))
  ;[1 1 1] Chase Player when seen
  (Utilities|FlowControl|Sequence
    (:then_0
      (Variables|Default|SetSeenPlayer true)
      (Variables|/Script/Engine.CharacterMovementComponent|SetMaxWalkSpeed (Variables|Character|GetCharacterMovement) 4e+02)
      (AI|AIMoveTo self "0, 0, 0" Pawn 5.0 false))
    (:then_1
      (Utilities|FlowControl|RetriggerableDelay 3.0)
      (CallFunction|ZombieRoam))))

(event OnTargetPerceptionUpdated(AIPerception)
  (params (Actor :type Actor%20Object%20Reference) (Stimulus :type AI%20Stimulus%20Structure))
  (bind (_age _expirationage _strength _stimuluslocation _receiverlocation _tag _bsuccessfullysensed) (Utilities|Struct|BreakAIStimulus Stimulus))
  ;[1 1 1] Move towards gunshot
  (Utilities|Casting|CastToBP_FirstPersonCharacter Actor)
  (if _bsuccessfullysensed
    (Variables|Default|SetSoundInvestigate true)
    (AI|AIMoveTo self _stimuluslocation 0 5.0 false
      (:OnSuccess
        (Utilities|FlowControl|Delay 2.0)
        (CallFunction|ZombieRoam)))))

(event OnComponentBeginOverlap(HitBox)
  (params (OverlappedComponent :type Primitive%20Component%20Object%20Reference) (OtherActor :type Actor%20Object%20Reference) (OtherComp :type Primitive%20Component%20Object%20Reference) (OtherBodyIndex :type Integer) (bFromSweep :type Boolean) (SweepResult :type Hit%20Result%20Structure%20%28by%20ref%29))
  ;[1 1 1] Damage Player
  (bind _asbp_first_person_character (Utilities|Casting|CastToBP_FirstPersonCharacter OtherActor))
  (if (== OtherActor _asbp_first_person_character)
    (Variables|Default|SetOverlappingPlayer true)
    (if (Variables|Default|GetOverlappingPlayer)
      (Game|Damage|ApplyDamage _asbp_first_person_character (Math|Conversions|ToFloat(Integer) (Math|Random|RandomIntegerinRange 10 15)) 0 self)
      (Variables|Default|SetAttacking true)
      (Utilities|FlowControl|Delay 0.5)
      (CallFunction|Attack))))

(event OnComponentEndOverlap(HitBox)
  (params (OverlappedComponent :type Primitive%20Component%20Object%20Reference) (OtherActor :type Actor%20Object%20Reference) (OtherComp :type Primitive%20Component%20Object%20Reference) (OtherBodyIndex :type Integer))
  ;[1 1 1] Update End Overlap
  (if (== OtherActor (Game|Player|GetPlayerPawn 0))
    (Variables|Default|SetAttacking false)
    (Variables|Default|SetOverlappingPlayer false)))

(event Custom|Zombie%20Roam
  ;[1 1 1] Random AI Roaming
  (AI|AIMoveTo self (.RandomLocation (AI|Navigation|GetRandomReachablePointinRadius (Transformation|GetActorLocation) 3e+03 0 0)) 0 5.0 false
    (:OnSuccess
      (Utilities|FlowControl|Delay (Math|Random|RandomFloatinRange 1.0 3.0)))
    (:OnFail
      _))
  (if (not (Variables|Default|GetSoundInvestigate))
    (CallFunction|ZombieRoam)))

(event Custom|SetHealth
  (Variables|Default|SetHealthCurrent (Variables|Default|GetHealthMax)))

(event Custom|Die
  (bind _returnvalue (Math|Random|RandomFloatinRange 0.0 1e+02))
  (bind _crit_box (Variables|Default|GetCrit%20Box))
  (bind _returnvalue_2 (Transformation|GetWorldTransform _crit_box))
  ;[1 1 1] Die
  (Variables|Default|SetZombieDead true)
  (Pawn|Components|CharacterMovement|DisableMovement (Variables|Character|GetCharacterMovement))
  (Utilities|FlowControl|Delay 2.0)
  (AI|SpawnAIFromClass "/Game/Blueprints/BP_ZombieSou.BP_ZombieSou_C" 0 (Transformation|GetWorldLocation (Variables|Default|GetCrit%20Box)) "0, 0, 0" false 0)
  (Utilities|FlowControl|Delay 0.2)
  (if (> _returnvalue 66.0)
    (Game|SpawnActorfromClass "/Game/Blueprints/ZombieStuff/Ammo/Mp5Ammo.Mp5Ammo_C" _returnvalue_2 "Undefined" "MultiplyWithRoot" 0 0)
    (elif (<= _returnvalue 33.0)
      (Game|SpawnActorfromClass "/Game/Blueprints/ZombieStuff/Ammo/PistolAmmo.PistolAmmo_C" _returnvalue_2 "Undefined" "MultiplyWithRoot" 0 0)))
  (Actor|DestroyActor))

(event Custom|Attack
  ;[1 1 1] Damage Player
  (if (Variables|Default|GetOverlappingPlayer)
    (Game|Damage|ApplyDamage (stale OnComponentBeginOverlap(HitBox) _asbp_first_person_character) (Math|Conversions|ToFloat(Integer) (Math|Random|RandomIntegerinRange 10 15)) 0 self)
    (Variables|Default|SetAttacking true)
    (Utilities|FlowControl|Delay 0.5)
    (CallFunction|Attack)))

(event EventBeginPlay
  (CallFunction|SetHealth)
  (CallFunction|ZombieRoam))

(event Game|Damage|EventAnyDamage
  (params (Damage :type Float%20%28single-precision%29) (DamageType :type Damage%20Type%20Object%20Reference) (InstigatedBy :type Controller%20Object%20Reference) (DamageCauser :type Actor%20Object%20Reference))
  ;[1 1 1] Recieve Damage
  (if (not (Variables|Default|GetZombieDead))
    (bind _output_get (Variables|Default|SetHealthCurrent (Math|Float|Clamp(Float) (- (Variables|Default|GetHealthCurrent) Damage) 0.0 (Variables|Default|GetHealthMax))))
    (if (== _output_get 0.0)
      (Audio|PlaySoundatLocation 0 (Transformation|GetActorLocation) "0, 0, 0" 1.0 1.0 0.0 0 0 0 0) ; Death SFX
      (Variables|Default|SetZombieDead true) ; Death animation plays after this
      (CallFunction|Die)
      (else
        (Audio|PlaySoundatLocation 0 (Transformation|GetActorLocation) "0, 0, 0" 1.0 1.0 0.0 0 0 0 0) ; Damage SFX
      ))))

(fn ConstructionScript)