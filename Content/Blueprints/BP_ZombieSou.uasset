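; BP_ZombieSou is an AI-moved pawn with a Niagara effect, apparently a zombie soul, that travels to BP_Artifact and notifies it via ZombieDies.
; On BeginPlay it caches the artifact, waits briefly, then runs AIMoveTo toward the artifact's Box location.
; Arrival calls ZombieDies, deactivates the effect and destroys the actor after a delay; a failed move only prints a message.
; A Collider hit on the artifact also calls ZombieDies, destroying the actor immediately.
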(event OnComponentHit(Collider)
  (params (HitComponent :type Primitive%20Component%20Object%20Reference) (OtherActor :type Actor%20Object%20Reference) (OtherComp :type Primitive%20Component%20Object%20Reference) (NormalImpulse :type Vector :default "0, 0, 0") (Hit :type Hit%20Result%20Structure%20%28by%20ref%29))
  (if (== (Variables|Default|GetArtifactRef) OtherActor)
    (Default|ZombieDies (Variables|Default|GetArtifactRef))
    (Actor|DestroyActor)))

(event EventBeginPlay
  (bind _returnvalue (Actor|GetActorOfClass "/Game/Blueprints/Artifact/BP_Artifact.BP_Artifact_C"))
  (Variables|Default|SetArtifactRef _returnvalue)
  (Utilities|FlowControl|Delay 0.5)
  (AI|AIMoveTo self (Transformation|GetWorldLocation (Variables|/Game/Blueprints/Artifact/BP_Artifact.BP_Artifact_C|GetBox _returnvalue)) 0 5.0 false
    (:OnSuccess
      (Default|ZombieDies (Variables|Default|GetArtifactRef))
      (Components|Activation|Deactivate (Variables|Default|GetNiagara))
      (Utilities|FlowControl|Delay 5.0)
      (Actor|DestroyActor))
    (:OnFail
      (Development|PrintString "TooSHort"))))

(event Collision|EventActorBeginOverlap
  (params (OtherActor :type Actor%20Object%20Reference)))

(event EventTick
  (params (DeltaSeconds :type Float%20%28single-precision%29)))

(fn ConstructionScript)