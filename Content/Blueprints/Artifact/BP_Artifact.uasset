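; Artifact actor that counts down zombie deaths as collected souls and gates the end of the game.
; ZombieDies decrements the remaining counter and plays the Artifact animation.
; When the player overlaps the box, a zero counter plus a distance check shows a reused EndtheGame widget and sets Endable, while a remaining count creates a new MoreSouls widget.
; Leaving the box hides both widgets and clears Endable.
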(event OnComponentBeginOverlap(Box)
  (params (OverlappedComponent :type Primitive%20Component%20Object%20Reference) (OtherActor :type Actor%20Object%20Reference) (OtherComp :type Primitive%20Component%20Object%20Reference) (OtherBodyIndex :type Integer) (bFromSweep :type Boolean) (SweepResult :type Hit%20Result%20Structure%20%28by%20ref%29))
  ;[1 1 1] Update Viewport
  (if (== OtherActor (Game|Player|GetPlayerPawn 0))
    (if (<= (Variables|Default|GetZombieCounters%20Left) 0.0)
      (if (<= (Math|Vector|Distance(Vector) (Transformation|GetWorldLocation (Variables|/Script/Engine.Character|GetCapsuleComponent (Variables|Default|GetAs%20BP%20First%20Person%20Character))) (Transformation|GetWorldLocation (Variables|Default|GetArtifact))) 5e+02)
        (if (Variables|Default|GetMadeWidget)
          (Widget|SetVisibility (Variables|Default|GetWidget) "Visible")
          (else
            (bind _returnvalue (UserInterface|CreateWidget "/Game/Blueprints/Artifact/EndtheGame.EndtheGame_C" (Game|GetPlayerController 0)))
            (bind _output_get (Variables|Default|SetWidget _returnvalue))
            (UserInterface|Viewport|AddtoViewport _output_get 0)
            (Variables|Default|SetMadeWidget true)))
        (Variables|Default|SetEndable true))
      (else
        (bind _returnvalue_2 (UserInterface|CreateWidget "/Game/Blueprints/Artifact/MoreSouls.MoreSouls_C" (Game|GetPlayerController 0)))
        (bind _output_get_2 (Variables|Default|SetMoreSouls%20Widget _returnvalue_2))
        (UserInterface|Viewport|AddtoViewport _output_get_2 0)))))

(event OnComponentEndOverlap(Box)
  (params (OverlappedComponent :type Primitive%20Component%20Object%20Reference) (OtherActor :type Actor%20Object%20Reference) (OtherComp :type Primitive%20Component%20Object%20Reference) (OtherBodyIndex :type Integer))
  ;[1 1 1] Hide Viewport when Leaving
  (if (== OtherActor (Game|Player|GetPlayerPawn 0))
    (Widget|SetVisibility (Variables|Default|GetWidget) "Hidden")
    (Widget|SetVisibility (Variables|Default|GetMoreSouls%20Widget) "Hidden")
    (Variables|Default|SetEndable false)))

(event Custom|ZombieDies
  ;[1 1 1] Update Zombie Counter
  (Variables|Default|SetZombieCounters%20Left (- (Variables|Default|GetZombieCounters%20Left) 1.0))
  (Components|Animation|PlayAnimation (Variables|Default|GetArtifact) 0 false)
  (Development|PrintString "SoildCollected"))

(event EventBeginPlay
  (bind _asbp_first_person_character (Utilities|Casting|CastToBP_FirstPersonCharacter (Game|Player|GetPlayerPawn 0)))
  (Variables|Default|SetAs%20BP%20First%20Person%20Character _asbp_first_person_character))

(fn ConstructionScript)