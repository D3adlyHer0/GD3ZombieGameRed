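; BP_1911 is a 1911 pistol actor that fires a hitscan shot when its PistolFire event is called.
; PistolFire starts the fire montage on the skeletal mesh, then immediately traces a short Visibility line forward from an Arrow component, with persistent debug drawing.
; The hit actor takes random damage, in a doubled range when the hit component's object name is "Crit Box".
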(event Custom|PistolFire
  (bind _arrow (Variables|Default|GetArrow))
  (bind _returnvalue (Transformation|GetWorldLocation _arrow))
  (Animation|Montage|PlayMontage (Variables|Default|GetSkeletalMesh) "/Game/Weapons/1911/Animations/1911Fire_Anim_Body_Fire_Montage.1911Fire_Anim_Body_Fire_Montage"
    (:then
      (bind _outhit (Collision|LineTraceByChannel _returnvalue (+ _returnvalue (* (Math|Vector|GetForwardVector (Transformation|GetWorldRotation _arrow)) (Math|Conversions|ToVector(Float) 1e+03))) "TraceTypeQuery1" false 0 "Persistent"))
      (if (Utilities|Enum|Equal(Enum) (Utilities|GetObjectName (.HitComponent (Collision|BreakHitResult _outhit))) "Crit Box")
        (Game|Damage|ApplyDamage (.HitActor (Collision|BreakHitResult _outhit)) (Math|Random|RandomFloatinRange 2e+01 3e+01) 0 0)
        (else
          (Game|Damage|ApplyDamage (.HitActor (Collision|BreakHitResult _outhit)) (Math|Random|RandomFloatinRange 1e+01 15.0) 0 0))))))

(event EventBeginPlay)

(event Collision|EventActorBeginOverlap
  (params (OtherActor :type Actor%20Object%20Reference)))

(event EventTick
  (params (DeltaSeconds :type Float%20%28single-precision%29)))

(event Input|MouseEvents|LeftMouseButton
  (params (Key :type Key%20Structure :default "None")))

(fn ConstructionScript)